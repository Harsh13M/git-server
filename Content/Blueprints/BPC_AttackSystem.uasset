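; Attack component for BP_ThirdPersonCharacter that runs a four-step melee combo of sword montages with a kick as the third hit.
; IA_Attack calls SwordAttack, which starts the montage for the current AttackIndex, or buffers the press in SaveAttack during an attack.
; Each attack advances the index behind a DoOnce guard.
; SwordAttackCombo, triggered from outside this graph, consumes the buffered press to continue the chain or calls StopCombo to reset it.
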(event Custom|Sword%20Attack
  ;[0.04057 0.02755 0.15 0.5] Sword Attack
  (if (Variables|Default|Getis%20Attacking?)
    (Variables|Default|SetSave%20Attack? true)
    (else
      (Variables|Default|Setis%20Attacking? true)
      (switch int (Variables|Default|GetAttack%20index)
        (:0
          (CallFunction|Attack1))
        (:1
          (CallFunction|Attack2))
        (:2
          (CallFunction|Attack3))
        (:3
          (CallFunction|Attack4))))))

(event Custom|SwordAttackCombo
  ;[0.03854 0.0288 0.15 0.5] Combo Continue
  (if (Variables|Default|GetSave%20Attack?)
    (Variables|Default|SetSave%20Attack? false)
    (switch int (Variables|Default|GetAttack%20index)
      (:0
        (CallFunction|Attack1))
      (:1
        (CallFunction|Attack2))
      (:2
        (CallFunction|Attack3))
      (:3
        (CallFunction|Attack4)))
    (else
      (CallFunction|StopCombo))))

(event Custom|Stop%20Combo
  ;[0.04816 0.02992 0.15 0.5] Stop Combo/Attack
  (Variables|Default|Setis%20Attacking? false)
  (Variables|Default|SetAttack%20index 0))

(event Custom|Attack%204
  ;[0.15 0.15 0.15 0.5] Attack 4
  (Utilities|FlowControl|DoOnce false :!label _label
    (:Completed
      (Utilities|FlowControl|Delay 0.1)
      (Animation|Montage|PlayMontage (Variables|Default|GetCharacter%20Mesh) "/Game/Characters/RPG_Character/Animation/SwordAttacks/Attack3_Montage.Attack3_Montage"
        (:then
          (Variables|Default|SetAttack%20index 4)
          (goto _label Reset))))))

(event Custom|Attack%201
  ;[0.15 0.15 0.15 0.5] Attack 1
  (Utilities|FlowControl|DoOnce false :!label _label
    (:Completed
      (Utilities|FlowControl|Delay 0.1)
      (Animation|Montage|PlayMontage (Variables|Default|GetCharacter%20Mesh) "/Game/Characters/RPG_Character/Animation/SwordAttacks/Attack1_Montage.Attack1_Montage"
        (:then
          (Variables|Default|SetAttack%20index 1)
          (goto _label Reset))))))

(event Custom|Attack%202
  ;[0.15 0.15 0.15 0.5] Attack 2
  (Utilities|FlowControl|DoOnce false :!label _label
    (:Completed
      (Utilities|FlowControl|Delay 0.1)
      (Animation|Montage|PlayMontage (Variables|Default|GetCharacter%20Mesh) "/Game/Characters/RPG_Character/Animation/SwordAttacks/Attack2_Montage.Attack2_Montage"
        (:then
          (Variables|Default|SetAttack%20index 2)
          (goto _label Reset))))))

(event Custom|Attack%203
  ;[0.15 0.15 0.15 0.5] Attack 3
  (Utilities|FlowControl|DoOnce false :!label _label
    (:Completed
      (Utilities|FlowControl|Delay 0.1)
      (Animation|Montage|PlayMontage (Variables|Default|GetCharacter%20Mesh) "/Game/Characters/RPG_Character/Animation/SwordAttacks/Kick_Montage.Kick_Montage"
        (:then
          (Variables|Default|SetAttack%20index 3)
          (goto _label Reset))))))

(event Input|EnhancedActionEvents|EnhancedInputActionIA_Attack
  (params (ActionValue :type Boolean) (ElapsedSeconds :type Float%20%28double-precision%29) (TriggeredSeconds :type Float%20%28double-precision%29) (InputAction :type Input%20Action%20Object%20Reference :default "/Game/ThirdPerson/Input/Actions/IA_Attack.IA_Attack"))
  ;[0.05374 0.03356 0.15 0.5] Attack Input
  (:Started
    (if (Variables|Default|GetCan%20Attack?)
      (CallFunction|SwordAttack))))

(event EventBeginPlay
  (bind _asbp_third_person_character (Utilities|Casting|CastToBP_ThirdPersonCharacter (Components|GetOwner)))
  (Variables|Default|SetCharacter%20Mesh (Variables|/Script/Engine.Character|GetMesh _asbp_third_person_character)))